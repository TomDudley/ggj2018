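; Game mode for a GGJ 2018 game that scores the player on time spent in the level.
; On BeginPlay it sets a full score and plays the calm electronic music cue at the player controller's mouse location.
; Tick drains the score at a steady rate, clamped at zero, and prints it on screen.
; GameEnded adds the remaining score to the running total in GGJGameInstance.
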(event Custom|Game%20Ended
  (bind _asggjgame_instance (Utilities|Casting|CastToGGJGameInstance (Game|GetGameInstance)))
  (Variables|/Game/Blueprints/GGJGameInstance.GGJGameInstance_C|SettotalPlayerScore _asggjgame_instance (+ (Variables|Default|GetPlayerScore) (Variables|/Game/Blueprints/GGJGameInstance.GGJGameInstance_C|GettotalPlayerScore _asggjgame_instance))))

(event EventBeginPlay
  (Variables|Default|SetScore%20deduction%20rate 1.0)
  (bind _output_get (Variables|Default|SetMax%20score 1e+03))
  (Variables|Default|SetPlayerScore _output_get)
  (bind _asggj_player_controller_bp (Utilities|Casting|CastToGGJ_PlayerControllerBP (Game|GetPlayerController 0)))
  (Audio|PlaySoundatLocation "/Game/Music/Calm_Electronic_Cue.Calm_Electronic_Cue" (Variables|/Game/Blueprints/Player/GGJ_PlayerControllerBP.GGJ_PlayerControllerBP_C|GetMouseLocation _asggj_player_controller_bp)))

(event EventTick
  (params (DeltaSeconds :type Float%20%28single-precision%29))
  (bind _output_get (Variables|Default|SetPlayerScore (Math|Float|Clamp(Float) (- (Variables|Default|GetPlayerScore) (* DeltaSeconds (Variables|Default|GetScore%20deduction%20rate))) 0.0 (Variables|Default|GetMax%20score))))
  (Development|PrintString (Utilities|String|ToString(Float) _output_get)))

(fn ConstructionScript)