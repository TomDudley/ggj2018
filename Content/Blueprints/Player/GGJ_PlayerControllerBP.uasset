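; Game jam player controller that lets the player place and rotate blocks (TestActor) with the mouse and keeps a score.
; Each tick traces under the cursor, accepting only Floor-tagged hits as placement points unless the left button is held.
; Pressing spawns a block with a sound; holding yaws it to point away from the cursor until release.
; AddScore adds to the score, optionally resetting it first.
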(event EventTick
  (params (DeltaSeconds :type Float%20%28single-precision%29))
  (bind (_worldlocation _worlddirection) (Game|Player|ConvertMouseLocationToWorldSpace))
  (bind _lastblock (Variables|Default|GetLastBlock))
  (bind (_outhit _returnvalue) (Collision|LineTraceByChannel _worldlocation (+ _worldlocation (* _worlddirection 1e+04)) "TraceTypeQuery1" false 0 "None"))
  (if _returnvalue
    ;[1 1 1] Set Mouse Coords
    (if (Game|Player|IsInputKeyDown "LeftMouseButton")
      (bind _output_get (Variables|Default|SetMouseLocation (.Location (Collision|BreakHitResult _outhit)) :!label _label))
      (elif (Actor|ActorHasTag (.HitActor (Collision|BreakHitResult _outhit)) "Floor")
        (goto _label)
        (else
          (Variables|Default|SetMouseLocation "0, 0, 0"))))
    ;[1 1 1] Set rotation
    (if (Game|Player|IsInputKeyDown "LeftMouseButton")
      (if (Utilities|IsValid _lastblock)
        (Transformation|SetActorRotation _lastblock (Math|Conversions|RotationFromXVector (Math|Vector|MakeVector (.X (Math|Vector|BreakVector (- (Transformation|GetActorLocation _lastblock) _output_get))) (.Y (Math|Vector|BreakVector (- (Transformation|GetActorLocation _lastblock) _output_get))) 0.0)) true)))))

(event Input|MouseEvents|LeftMouseButton
  (params (Key :type Key%20Structure))
  (:Pressed
    (if (not (Math|Vector|Equal(Vector) (Variables|Default|GetMouseLocation) "0, 0, 0" 0.0001))
      (bind _returnvalue (Game|SpawnActorfromClass "/Game/Blueprints/Player/TestActor.TestActor_C" (Math|Conversions|ToTransform(Vector) (Variables|Default|GetMouseLocation)) "Undefined" 0 0))
      (Variables|Default|SetLastBlock _returnvalue)
      (Audio|PlaySoundatLocation "/Game/Music/PlacementSounds.PlacementSounds" (Variables|Default|GetMouseLocation))))
  (:Released
    (Variables|Default|SetMouseLocation "0, 0, 0")
    (Variables|Default|SetLastBlock 0)))

(fn ConstructionScript)

(fn AddScore
  (params (AddScore :type Integer) (isReset :type Boolean))
  (if isReset
    (Variables|Default|SetScore 0))
  (Variables|Default|SetScore (+ AddScore (Variables|Default|GetScore))))