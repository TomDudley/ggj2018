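; Test actor for mouse-driven placement on floors, following the cursor and rotating while the left button is held.
; Each tick it deprojects the mouse from GGJ_PlayerControllerBP and line-traces on Visibility, acting only on hits tagged "Floor".
; Unclicked, it moves to the hit point; held, it yaws toward the hit point around its fixed position.
; Releasing the button resets rotation to zero, and it resumes following the cursor.
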(event EventTick
  (params (DeltaSeconds :type Float%20%28single-precision%29))
  (bind _asggj_player_controller_bp (Utilities|Casting|CastToGGJ_PlayerControllerBP (Game|GetPlayerController 0)))
  (bind (_outhit _returnvalue) (Collision|LineTraceByChannel (.WorldLocation (Game|Player|ConvertMouseLocationToWorldSpace _asggj_player_controller_bp)) (+ (.WorldLocation (Game|Player|ConvertMouseLocationToWorldSpace _asggj_player_controller_bp)) (* (.WorldDirection (Game|Player|ConvertMouseLocationToWorldSpace _asggj_player_controller_bp)) 1e+04)) "TraceTypeQuery1" false 0 "None"))
  (if _returnvalue
    (if (Actor|ActorHasTag (.HitActor (Collision|BreakHitResult _outhit)) "Floor")
      (if (Variables|Default|GetisLeftClicked)
        (Transformation|SetActorRotation (Math|Conversions|RotationFromXVector (Math|Vector|MakeVector (.X (Math|Vector|BreakVector (- (.Location (Collision|BreakHitResult _outhit)) (Transformation|GetActorLocation)))) (.Y (Math|Vector|BreakVector (- (.Location (Collision|BreakHitResult _outhit)) (Transformation|GetActorLocation)))) 0.0)))
        (else
          (Transformation|SetActorLocation (.Location (Collision|BreakHitResult _outhit)) false false))))))

(event EventBeginPlay
  (Input|EnableInput (Game|GetPlayerController 0)))

(event Input|MouseEvents|LeftMouseButton
  (params (Key :type Key%20Structure))
  (:Pressed
    (Variables|Default|SetisLeftClicked true))
  (:Released
    (Variables|Default|SetisLeftClicked false)
    (Transformation|SetActorRotation "0, 0, 0")))

(fn ConstructionScript)